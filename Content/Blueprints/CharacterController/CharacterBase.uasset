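; Base player character with movement, look and jump input, plus picking up and dropping items the player looks at.
; Every Tick, a debug-drawn line trace from the camera stores the ItemBase under view and its distance.
; Left mouse press picks up that item if it is a PickUpableItem in range, passing the camera as location actor; release drops the currently targeted item.
; Steam host and join calls are left unconnected.
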(event `InputAxis|MoveForward`
  (params (AxisValue :type "Float (single-precision)"))
  ;[1 1 1] Character movement and rotation
  (`self.AddMovementInput` (`self.GetActorForwardVector`) AxisValue))

(event `InputAxis|Turn`
  (params (AxisValue :type "Float (single-precision)"))
  ;[1 1 1] Character movement and rotation
  (`self.AddControllerYawInput` AxisValue))

(event `InputAxis|LookUp`
  (params (AxisValue :type "Float (single-precision)"))
  ;[1 1 1] Character movement and rotation
  (`self.AddControllerPitchInput` AxisValue))

(event `InputAxis|MoveRight`
  (params (AxisValue :type "Float (single-precision)"))
  ;[1 1 1] Character movement and rotation
  (`self.AddMovementInput` (`self.GetActorRightVector`) AxisValue))

(event `InputAction|Jump`
  (params (Key :type "Key Structure"))
  ;[1 1 1] Character movement and rotation
  (:`Pressed`
    (`self.Jump`)))

(event `self.ReceiveTick`
  (params (DeltaSeconds :type "Float (single-precision)"))
  (`self.Interact`))

(event `Interact`
  (bind _camera (`self.Camera`))
  (bind _returnvalue (`SceneComponent.K2_GetComponentLocation` _camera))
  ;[1 1 1] Interact
  (bind (_outhit _returnvalue_2) (`KismetSystemLibrary.LineTraceSingle` :`Start` _returnvalue :`End` (+ _returnvalue (* (`SceneComponent.GetForwardVector` _camera) (`KismetMathLibrary.FTrunc` (`self.MaxInteractDistance`)))) :`TraceChannel` "TraceTypeQuery1" :`DrawDebugType` "ForOneFrame"))
  (if _returnvalue_2
    (bind (_bblockinghit _binitialoverlap _time _distance _location _impactpoint _normal _impactnormal _physmat _hitactor) (`GameplayStatics.BreakHitResult` _outhit))
    (bind _asitem_base (cast `/Game/Blueprints/Items/ItemBase` _hitactor)
      (:`then`
        (set `self.CurrentItem` _asitem_base)
        (set `self.DistanceToItem` _distance))
      (:`CastFailed`
        (set `self.CurrentItem` null :!label _label)))
    (else
      (goto _label))))

(event `PickUpServer`
  ;[1 1 1] Pickup and Drop
  (bind _currentitem (`self.CurrentItem`)
    (:`then`
      (if (< (`self.DistanceToItem`) (`self.MaxInteractDistance`))
        (bind _aspick_upable_item (cast `/Game/Blueprints/Items/PickUpableItem` _currentitem))
        (`/Game/Blueprints/Items/PickUpableItem.PickUpServer` _aspick_upable_item (`self.Camera`) (`self.MaxInteractDistance`))))
    (:`else`)))

(event `Key|LeftMouseButton`
  (params (Key :type "Key Structure"))
  ;[1 1 1] Pickup and Drop
  (:`Pressed`
    (`self.PickUpServer`))
  (:`Released`
    (`self.DropServer`)))

(event `DropServer`
  ;[1 1 1] Pickup and Drop
  (bind _currentitem (`self.CurrentItem`)
    (:`then`
      (bind _aspick_upable_item (cast `/Game/Blueprints/Items/PickUpableItem` _currentitem))
      (`/Game/Blueprints/Items/PickUpableItem.Drop` _aspick_upable_item))
    (:`else`)))

(event `Key|H`
  (params (Key :type "Key Structure")))

(event `Key|J`
  (params (Key :type "Key Structure")))

(fn `UserConstructionScript`)