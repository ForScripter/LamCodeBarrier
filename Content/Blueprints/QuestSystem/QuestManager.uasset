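; QuestManager is a quest actor that activates target actors once every item in its CheckItems list reaches a required state.
; On BeginPlay it binds one shared handler to each item's state-change event.
; Each change rescans all items against a single enum value, calling UseItem on every ActivateActor entry if all match.
; Otherwise it resets the IsAllDone flag to true for the next check.
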(event `self.ReceiveBeginPlay`
  (for _array_element (`self.CheckItems`)
    (add `/Game/Blueprints/Items/ItemBase.StateChanged` _array_element (delegate `StateChanged_Event_0`))))

(event `StateChanged_Event_0`
  (for _array_element (`self.CheckItems`)
    (if (`|EnumInequality` (`/Game/Blueprints/Items/ItemBase.State` _array_element) "NewEnumerator2")
      (set `self.isAllDone` false)))
  (if (`self.isAllDone`)
    (for _array_element_2 (`self.ActivateActor`)
      (`/Game/Blueprints/Items/UsableItem.UseItem` _array_element_2))
    (else
      (set `self.isAllDone` true))))

(fn `UserConstructionScript`)