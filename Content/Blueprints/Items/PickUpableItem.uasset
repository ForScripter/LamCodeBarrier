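; PickUpableItem is a physics item actor that can be picked up, carried in front of a scene component and dropped.
; PickUpLocal forwards to PickUpServer, which turns off mesh physics and stores the holding component and distance.
; While held, Tick moves the actor along that component's forward vector by the truncated distance, without sweeping.
; Drop re-enables physics and clears the held flag.
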(event `self.ReceiveTick`
  (params (DeltaSeconds :type "Float (single-precision)"))
  (bind _locationactor (`self.LocationActor`))
  (`parent.ReceiveTick` DeltaSeconds)
  (if (`self.isPickedUp`)
    (`self.K2_SetActorLocation` (+ (`SceneComponent.K2_GetComponentLocation` _locationactor) (* (`SceneComponent.GetForwardVector` _locationactor) (`KismetMathLibrary.FTrunc` (`self.Distance`)))))))

(event `PickUpLocal`
  (params (LocationActor :type "CameraComponent Object Reference") (Distance :type "Float (double-precision)"))
  (`self.PickUpServer` LocationActor Distance))

(event `PickUpServer`
  (params (LocationActor :type "CameraComponent Object Reference") (Distance :type "Float (double-precision)"))
  (`PrimitiveComponent.SetSimulatePhysics` (`self.StaticMesh`) false)
  (set `self.isPickedUp` true)
  (set `self.LocationActor` LocationActor)
  (set `self.Distance` Distance)
  (`KismetSystemLibrary.PrintString` "pickup"))

(event `Drop`
  (`PrimitiveComponent.SetSimulatePhysics` (`self.StaticMesh`) true)
  (set `self.isPickedUp` false))

(fn `UserConstructionScript`
  (`parent.UserConstructionScript`))